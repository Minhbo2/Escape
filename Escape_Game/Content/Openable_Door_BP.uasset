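; An openable door actor that swings open and closed in response to OpenDoor's OnOpen and OnClose events.
; It stores its rotation at BeginPlay, and a timeline curve adds yaw to that rotation so the swing is relative to the door's placed orientation.
; OnOpen plays the timeline, OnClose reverses it, and an event track plays a door lock sound at the door's location.
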(event `self.ReceiveBeginPlay`
  ;[1 1 1] Get the actor initial rotation
  (set `self.Initial Rotation` (`self.K2_GetActorRotation`)) ; RCLK->Promote Variable
)

(event `self.OpenDoor.OnOpen`
  (bind (_direction _open_door_curve) (`Timeline|Timeline_0` :!label _label) ; Add TimeLine
    (:`Update`
      (`self.K2_SetActorRotation` (`KismetMathLibrary.ComposeRotators` (`KismetMathLibrary.MakeRotator` 0.0 0.0 _open_door_curve) (`self.Initial Rotation`))))
    (:`Sound Event`
      (`GameplayStatics.PlaySoundAtLocation` "/Game/door-lock.door-lock" (`self.K2_GetActorLocation`)))))

(event `self.OpenDoor.OnClose`
  (goto _label :!via `Reverse`))

(fn `UserConstructionScript`)